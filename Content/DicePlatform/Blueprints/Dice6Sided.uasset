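; Six-sided dice platform Blueprint that reveals a timed chain of steps, with faces 5 down to 1 hidden and non-collidable at start.
; Each trigger from 6 down to 2 fires once, in order, revealing and enabling collision on the next face.
; If the following trigger is not reached within the Time delay, revealed faces hide and ResetDice re-arms the DoOnce gates.
; The last step always resets after its delay.
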(event OnComponentBeginOverlap(TriggerDi6)
  (params (OverlappedComponent :type Primitive%20Component%20Object%20Reference) (OtherActor :type Actor%20Object%20Reference) (OtherComp :type Primitive%20Component%20Object%20Reference) (OtherBodyIndex :type Integer) (bFromSweep :type Boolean) (SweepResult :type Hit%20Result%20Structure%20%28by%20ref%29))
  (bind _di5 (Variables|Default|GetDi5))
  (bind _di4 (Variables|Default|GetDi4))
  (bind _di5_2 (Variables|Default|GetDi5))
  (bind _si3 (Variables|Default|GetSi3))
  (bind _si2 (Variables|Default|GetSi2))
  (bind _di1 (Variables|Default|GetDi1))
  (Utilities|FlowControl|DoOnce false
    (:Completed
      (Rendering|ToggleVisibility _di5 false)
      (Collision|SetCollisionEnabled _di5 "QueryAndPhysics")
      (Variables|Default|SetDi6Triggered true)
      (Utilities|FlowControl|Delay (Variables|Default|GetTime))
      (if (not (Variables|Default|GetDi5Triggered))
        (Collision|SetCollisionEnabled _di5_2 "NoCollision")
        (Utilities|FlowControl|Sequence
          (:then_0
            (if (Rendering|IsVisible _di5_2)
              (Rendering|ToggleVisibility _di5_2 false)
              (CallFunction|ResetDice :!label _label)
              (Variables|Default|SetDi6Triggered false)
              (Variables|Default|SetDi5Triggered false)
              (Variables|Default|SetDi4Triggered false)
              (Variables|Default|SetDi3Triggered false)
              (Variables|Default|SetDi2Triggered false)))
          (:then_1
            (if (Rendering|IsVisible _di4)
              (Rendering|ToggleVisibility _di4 false)
              (goto _label)))
          (:then_2
            (if (Rendering|IsVisible _si3)
              (Rendering|ToggleVisibility _si3 false)
              (goto _label)))
          (:then_3
            (if (Rendering|IsVisible _si2)
              (Rendering|ToggleVisibility _si2 false)
              (goto _label)))
          (:then_4
            (if (Rendering|IsVisible _di1)
              (Rendering|ToggleVisibility _di1 false)
              (goto _label))))))))

(event OnComponentBeginOverlap(TriggerDi5)
  (params (OverlappedComponent :type Primitive%20Component%20Object%20Reference) (OtherActor :type Actor%20Object%20Reference) (OtherComp :type Primitive%20Component%20Object%20Reference) (OtherBodyIndex :type Integer) (bFromSweep :type Boolean) (SweepResult :type Hit%20Result%20Structure%20%28by%20ref%29))
  (bind _di4 (Variables|Default|GetDi4))
  (bind _di4_2 (Variables|Default|GetDi4))
  (bind _di5 (Variables|Default|GetDi5))
  (bind _si3 (Variables|Default|GetSi3))
  (bind _si2 (Variables|Default|GetSi2))
  (bind _di1 (Variables|Default|GetDi1))
  (if (Variables|Default|GetDi6Triggered)
    (Utilities|FlowControl|DoOnce false
      (:Completed
        (Rendering|ToggleVisibility _di4_2 false)
        (Collision|SetCollisionEnabled _di4_2 "QueryAndPhysics")
        (Variables|Default|SetDi5Triggered true)
        (Utilities|FlowControl|Delay (Variables|Default|GetTime))
        (if (not (Variables|Default|GetDi4Triggered))
          (Collision|SetCollisionEnabled _di5 "NoCollision")
          (Utilities|FlowControl|Sequence
            (:then_0
              (if (Rendering|IsVisible _di5)
                (Rendering|ToggleVisibility _di5 false)
                (CallFunction|ResetDice :!label _label)
                (Variables|Default|SetDi6Triggered false)
                (Variables|Default|SetDi5Triggered false)
                (Variables|Default|SetDi4Triggered false)
                (Variables|Default|SetDi3Triggered false)
                (Variables|Default|SetDi2Triggered false)))
            (:then_1
              (if (Rendering|IsVisible _di4)
                (Rendering|ToggleVisibility _di4 false)
                (goto _label)))
            (:then_2
              (if (Rendering|IsVisible _si3)
                (Rendering|ToggleVisibility _si3 false)
                (goto _label)))
            (:then_3
              (if (Rendering|IsVisible _si2)
                (Rendering|ToggleVisibility _si2 false)
                (goto _label)))
            (:then_4
              (if (Rendering|IsVisible _di1)
                (Rendering|ToggleVisibility _di1 false)
                (goto _label)))))))))

(event OnComponentBeginOverlap(TriggerDi4)
  (params (OverlappedComponent :type Primitive%20Component%20Object%20Reference) (OtherActor :type Actor%20Object%20Reference) (OtherComp :type Primitive%20Component%20Object%20Reference) (OtherBodyIndex :type Integer) (bFromSweep :type Boolean) (SweepResult :type Hit%20Result%20Structure%20%28by%20ref%29))
  (bind _di4 (Variables|Default|GetDi4))
  (bind _di5 (Variables|Default|GetDi5))
  (bind _si3 (Variables|Default|GetSi3))
  (bind _si2 (Variables|Default|GetSi2))
  (bind _di1 (Variables|Default|GetDi1))
  (bind _si3_2 (Variables|Default|GetSi3))
  (if (Variables|Default|GetDi5Triggered)
    (Utilities|FlowControl|DoOnce false
      (:Completed
        (Rendering|ToggleVisibility _si3_2 false)
        (Collision|SetCollisionEnabled _si3_2 "QueryAndPhysics")
        (Variables|Default|SetDi4Triggered true)
        (Utilities|FlowControl|Delay (Variables|Default|GetTime))
        (if (not (Variables|Default|GetDi3Triggered))
          (Collision|SetCollisionEnabled _di5 "NoCollision")
          (Utilities|FlowControl|Sequence
            (:then_0
              (if (Rendering|IsVisible _di5)
                (Rendering|ToggleVisibility _di5 false)
                (CallFunction|ResetDice :!label _label)
                (Variables|Default|SetDi6Triggered false)
                (Variables|Default|SetDi5Triggered false)
                (Variables|Default|SetDi4Triggered false)
                (Variables|Default|SetDi3Triggered false)
                (Variables|Default|SetDi2Triggered false)))
            (:then_1
              (if (Rendering|IsVisible _di4)
                (Rendering|ToggleVisibility _di4 false)
                (goto _label)))
            (:then_2
              (if (Rendering|IsVisible _si3)
                (Rendering|ToggleVisibility _si3 false)
                (goto _label)))
            (:then_3
              (if (Rendering|IsVisible _si2)
                (Rendering|ToggleVisibility _si2 false)
                (goto _label)))
            (:then_4
              (if (Rendering|IsVisible _di1)
                (Rendering|ToggleVisibility _di1 false)
                (goto _label)))))))))

(event OnComponentBeginOverlap(TriggerDi3)
  (params (OverlappedComponent :type Primitive%20Component%20Object%20Reference) (OtherActor :type Actor%20Object%20Reference) (OtherComp :type Primitive%20Component%20Object%20Reference) (OtherBodyIndex :type Integer) (bFromSweep :type Boolean) (SweepResult :type Hit%20Result%20Structure%20%28by%20ref%29))
  (bind _di4 (Variables|Default|GetDi4))
  (bind _di5 (Variables|Default|GetDi5))
  (bind _si3 (Variables|Default|GetSi3))
  (bind _si2 (Variables|Default|GetSi2))
  (bind _di1 (Variables|Default|GetDi1))
  (bind _si2_2 (Variables|Default|GetSi2))
  (if (Variables|Default|GetDi4Triggered)
    (Utilities|FlowControl|DoOnce false
      (:Completed
        (Rendering|ToggleVisibility _si2_2 false)
        (Collision|SetCollisionEnabled _si2_2 "QueryAndPhysics")
        (Variables|Default|SetDi3Triggered true)
        (Utilities|FlowControl|Delay (Variables|Default|GetTime))
        (if (not (Variables|Default|GetDi2Triggered))
          (Collision|SetCollisionEnabled _di5 "NoCollision")
          (Utilities|FlowControl|Sequence
            (:then_0
              (if (Rendering|IsVisible _di5)
                (Rendering|ToggleVisibility _di5 false)
                (CallFunction|ResetDice :!label _label)
                (Variables|Default|SetDi6Triggered false)
                (Variables|Default|SetDi5Triggered false)
                (Variables|Default|SetDi4Triggered false)
                (Variables|Default|SetDi3Triggered false)
                (Variables|Default|SetDi2Triggered false)))
            (:then_1
              (if (Rendering|IsVisible _di4)
                (Rendering|ToggleVisibility _di4 false)
                (goto _label)))
            (:then_2
              (if (Rendering|IsVisible _si3)
                (Rendering|ToggleVisibility _si3 false)
                (goto _label)))
            (:then_3
              (if (Rendering|IsVisible _si2)
                (Rendering|ToggleVisibility _si2 false)
                (goto _label)))
            (:then_4
              (if (Rendering|IsVisible _di1)
                (Rendering|ToggleVisibility _di1 false)
                (goto _label)))))))))

(event OnComponentBeginOverlap(TriggerDi2)
  (params (OverlappedComponent :type Primitive%20Component%20Object%20Reference) (OtherActor :type Actor%20Object%20Reference) (OtherComp :type Primitive%20Component%20Object%20Reference) (OtherBodyIndex :type Integer) (bFromSweep :type Boolean) (SweepResult :type Hit%20Result%20Structure%20%28by%20ref%29))
  (bind _di4 (Variables|Default|GetDi4))
  (bind _di5 (Variables|Default|GetDi5))
  (bind _si3 (Variables|Default|GetSi3))
  (bind _si2 (Variables|Default|GetSi2))
  (bind _di1 (Variables|Default|GetDi1))
  (bind _di1_2 (Variables|Default|GetDi1))
  (if (Variables|Default|GetDi3Triggered)
    (Utilities|FlowControl|DoOnce false
      (:Completed
        (Rendering|ToggleVisibility _di1_2 false)
        (Collision|SetCollisionEnabled _di1_2 "QueryAndPhysics")
        (Variables|Default|SetDi2Triggered true)
        (Utilities|FlowControl|Delay (Variables|Default|GetTime))
        (Collision|SetCollisionEnabled _di5 "NoCollision")
        (Utilities|FlowControl|Sequence
          (:then_0
            (if (Rendering|IsVisible _di5)
              (Rendering|ToggleVisibility _di5 false)
              (CallFunction|ResetDice :!label _label)
              (Variables|Default|SetDi6Triggered false)
              (Variables|Default|SetDi5Triggered false)
              (Variables|Default|SetDi4Triggered false)
              (Variables|Default|SetDi3Triggered false)
              (Variables|Default|SetDi2Triggered false)))
          (:then_1
            (if (Rendering|IsVisible _di4)
              (Rendering|ToggleVisibility _di4 false)
              (goto _label)))
          (:then_2
            (if (Rendering|IsVisible _si3)
              (Rendering|ToggleVisibility _si3 false)
              (goto _label)))
          (:then_3
            (if (Rendering|IsVisible _si2)
              (Rendering|ToggleVisibility _si2 false)
              (goto _label)))
          (:then_4
            (if (Rendering|IsVisible _di1)
              (Rendering|ToggleVisibility _di1 false)
              (goto _label))))))))

(event Custom|ResetDice
  (bind _di5 (Variables|Default|GetDi5))
  (bind _di4 (Variables|Default|GetDi4))
  (bind _di4_2 (Variables|Default|GetDi4))
  (bind _di5_2 (Variables|Default|GetDi5))
  (bind _si3 (Variables|Default|GetSi3))
  (bind _si2 (Variables|Default|GetSi2))
  (bind _di1 (Variables|Default|GetDi1))
  (bind _si3_2 (Variables|Default|GetSi3))
  (bind _si2_2 (Variables|Default|GetSi2))
  (bind _di1_2 (Variables|Default|GetDi1))
  (Utilities|FlowControl|Sequence
    (:then_0
      (Utilities|FlowControl|DoOnce false) ; enters at Reset
    )
    (:then_1
      (Utilities|FlowControl|DoOnce false) ; enters at Reset
    )
    (:then_2
      (Utilities|FlowControl|DoOnce false) ; enters at Reset
    )
    (:then_3
      (Utilities|FlowControl|DoOnce false) ; enters at Reset
    )
    (:then_4
      (Utilities|FlowControl|DoOnce false) ; enters at Reset
    )))

(event EventBeginPlay
  (bind _di5 (Variables|Default|GetDi5))
  (Rendering|ToggleVisibility _di5 false)
  (Collision|SetCollisionEnabled _di5 "NoCollision"))

(event Collision|EventActorBeginOverlap
  (params (OtherActor :type Actor%20Object%20Reference)))

(event EventTick
  (params (DeltaSeconds :type Float%20%28single-precision%29)))

(fn ConstructionScript)