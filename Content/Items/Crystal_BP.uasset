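; Crystal_BP is a crystal item that swaps its look and tracks whether something has entered its singing range.
; One second after BeginPlay it picks one of two skeletal mesh materials based on InBoardGameBox.
; Overlapping CollectSphere sets its own InRangeForSinging flag, with no live path to clear it.
; The Bob timeline motion and Rad_Blueprint player flag updates are disconnected, and SetHidden has no effect.
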(event OnComponentBeginOverlap(CollectSphere)
  (params (OverlappedComponent :type Primitive%20Component%20Object%20Reference) (OtherActor :type Actor%20Object%20Reference) (OtherComp :type Primitive%20Component%20Object%20Reference) (OtherBodyIndex :type Integer) (bFromSweep :type Boolean) (SweepResult :type Hit%20Result%20Structure%20%28by%20ref%29))
  (Variables|Default|SetIn%20Range%20For%20Singing true))

(event EventBeginPlay
  (bind _skeletalmesh (Variables|Default|GetSkeletalMesh))
  (Utilities|FlowControl|Delay 1.0)
  (if (Variables|Default|GetInBoardGameBox)
    (Rendering|Material|SetMaterial _skeletalmesh 0 "/Game/Geometry/Meshes/Items/Materials/Crystal_Diff_Mat2.Crystal_Diff_Mat2")
    (else
      (Rendering|Material|SetMaterial _skeletalmesh 0 "/Game/Geometry/Meshes/Items/Materials/Crystal_Diff_Mat.Crystal_Diff_Mat"))))

(event EventTick
  (params (DeltaSeconds :type Float%20%28single-precision%29)))

(fn ConstructionScript)

(fn SetHidden
  (params (NewHidden :type Boolean))
  (if NewHidden
    _))