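; Board game box pickup that rewards Rad with a crystal once he has collected 100 coins.
; BeginPlay uses Rad's level number to show the Sorry or cards box and matching count sign, then sets a Collect100 placeholder crystal.
; Entering the sphere with enough coins swaps in the collidable crystal once; leaving reveals the sign and stars.
; Tick yaws the sign toward the player, with a -90 degree offset overriding the first rotation.
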(event OnComponentBeginOverlap(Sphere)
  (params (OverlappedComponent :type Primitive%20Component%20Object%20Reference) (OtherActor :type Actor%20Object%20Reference) (OtherComp :type Primitive%20Component%20Object%20Reference) (OtherBodyIndex :type Integer) (bFromSweep :type Boolean) (SweepResult :type Hit%20Result%20Structure%20%28by%20ref%29))
  (Utilities|FlowControl|Sequence
    (:then_0
      (bind _asrad_blueprint (Utilities|Casting|CastToRad_Blueprint OtherActor))
      (if (>= (Variables|/Game/ThirdPersonBP/Blueprints/Rad_Blueprint.Rad_Blueprint_C|GetCoin%20Count _asrad_blueprint) 100)
        (Utilities|FlowControl|DoOnce false
          (:Completed
            (Collision|SetActorEnableCollision (Variables|/Script/Engine.ChildActorComponent|GetChildActor (Variables|Default|GetCrystal_BP)) true)
            (ChildActorComponent|SetChildActorClass (Variables|Default|GetCrystal_BP) "/Game/Items/Crystal_BP.Crystal_BP_C")
            (Rendering|SetVisibility (Variables|Default|GetCrystal_BP) true true)))))))

(event OnComponentEndOverlap(Sphere)
  (params (OverlappedComponent :type Primitive%20Component%20Object%20Reference) (OtherActor :type Actor%20Object%20Reference) (OtherComp :type Primitive%20Component%20Object%20Reference) (OtherBodyIndex :type Integer))
  (Development|SetHiddeninGame (Variables|Default|GetHowManyCoins) false false))

(event Custom|Find%20Level
  (bind _howmanycoins (Variables|Default|GetHowManyCoins))
  (Utilities|FlowControl|Sequence
    (:then_0
      (bind _asrad_blueprint (Utilities|Casting|CastToRad_Blueprint (Game|GetPlayerCharacter 0)))
      (if (== (Variables|/Game/ThirdPersonBP/Blueprints/Rad_Blueprint.Rad_Blueprint_C|GetLevel%20Number _asrad_blueprint) 1)
        (Development|SetHiddeninGame (Variables|Default|GetBoardGameBox_Cards_Anim) false false)
        (Rendering|Material|SetMaterial _howmanycoins 0 "/Game/Geometry/Meshes/Items/Materials/HowManyCards_Diff_Mat.HowManyCards_Diff_Mat")))
    (:then_1
      (bind _asrad_blueprint_2 (Utilities|Casting|CastToRad_Blueprint (Game|GetPlayerCharacter 0)))
      (if (== (Variables|/Game/ThirdPersonBP/Blueprints/Rad_Blueprint.Rad_Blueprint_C|GetLevel%20Number _asrad_blueprint_2) 0)
        (Development|SetHiddeninGame (Variables|Default|GetBoardGameBox_Sorry_Anim) false false)
        (Rendering|Material|SetMaterial _howmanycoins 0 "/Game/Geometry/Meshes/Items/Materials/HowManyPawns_Diff_Mat.HowManyPawns_Diff_Mat")))))

(event EventBeginPlay
  (Utilities|FlowControl|Sequence
    (:then_0
      ;[1 1 1] Give Crystal
      (Collision|SetActorEnableCollision (Variables|/Script/Engine.ChildActorComponent|GetChildActor (Variables|Default|GetCrystal_BP)) false))
    (:then_1
      (CallFunction|FindLevel))
    (:then_2
      (ChildActorComponent|SetChildActorClass (Variables|Default|GetCrystal_BP) "/Game/Items/Crystal_BP_Collect100.Crystal_BP_Collect100_C"))))

(event EventTick
  (params (DeltaSeconds :type Float%20%28single-precision%29))
  (bind _howmanycoins (Variables|Default|GetHowManyCoins))
  (Utilities|FlowControl|Sequence
    (:then_0
      ;[1 1 1] Rotate Towards Rad
      (Utilities|FlowControl|Sequence
        (:then_0
          (Transformation|SetWorldRotation _howmanycoins (Math|Rotator|MakeRotator 0.0 0.0 (+ (.Yaw (Math|Rotator|BreakRotator (Math|Rotator|FindLookatRotation (Transformation|GetActorLocation) (Transformation|GetActorLocation (Game|GetPlayerCharacter 0))))) 0.0)) false false))
        (:then_1
          (Transformation|SetWorldRotation _howmanycoins (Math|Rotator|MakeRotator 0.0 0.0 (+ (.Yaw (Math|Rotator|BreakRotator (Math|Rotator|FindLookatRotation (Transformation|GetActorLocation) (Transformation|GetActorLocation (Game|GetPlayerCharacter 0))))) -9e+01)) false false))))))

(fn ConstructionScript)