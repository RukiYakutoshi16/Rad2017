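; SingingRad_BP is an item that makes the player's controller rumble while the player is within its singing range.
; Overlapping the SingingRange component starts a looping Rad_Singing force feedback effect on the first player's controller, and ending the overlap stops it.
; The InSingRange flag follows begin and end overlaps from any actor, while the rumble responds only to the player character.
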(event OnComponentBeginOverlap(SingingRange)
  (params (OverlappedComponent :type Primitive%20Component%20Object%20Reference) (OtherActor :type Actor%20Object%20Reference) (OtherComp :type Primitive%20Component%20Object%20Reference) (OtherBodyIndex :type Integer) (bFromSweep :type Boolean) (SweepResult :type Hit%20Result%20Structure%20%28by%20ref%29))
  (Variables|Default|SetInSingRange true)
  (if (== OtherActor (Game|GetPlayerCharacter 0))
    (Game|Feedback|ClientPlayForceFeedback (Game|GetPlayerController 0) "/Game/Items/Rad_Singing.Rad_Singing" true "None")))

(event OnComponentEndOverlap(SingingRange)
  (params (OverlappedComponent :type Primitive%20Component%20Object%20Reference) (OtherActor :type Actor%20Object%20Reference) (OtherComp :type Primitive%20Component%20Object%20Reference) (OtherBodyIndex :type Integer))
  (Variables|Default|SetInSingRange false)
  (if (== OtherActor (Game|GetPlayerCharacter 0))
    (Game|Feedback|ClientStopForceFeedback (Game|GetPlayerController 0) "/Game/Items/Rad_Singing.Rad_Singing" "None")))

(fn ConstructionScript)