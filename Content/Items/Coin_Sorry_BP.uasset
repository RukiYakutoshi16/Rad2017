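; Coin item Blueprint that sets its look from the player character's TypeofCoin, with no pickup logic in this graph.
; After a short BeginPlay delay, it reads Rad_Blueprint and toggles on the Sorry, Card or Die component; the Letters and Evidence branches are empty.
; RandomTexture randomizes the Sorry material or Die mesh, with a zero roll keeping the default.
; Tick spins the die at a fixed per-frame rate while DiceOn is set.
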(event EventTick
  (params (DeltaSeconds :type Float%20%28single-precision%29))
  (Utilities|FlowControl|Sequence
    (:then_0
      (if (Variables|Default|GetDiceOn)
        (Transformation|AddRelativeRotation (Variables|Default|GetDie) "0.000000,2.000000,2.000000" false false)))))

(event EventBeginPlay
  (bind _sorry (Variables|Default|GetSorry))
  (bind _die (Variables|Default|GetDie))
  (Utilities|FlowControl|Delay 0.8)
  (bind _asrad_blueprint (Utilities|Casting|CastToRad_Blueprint (Game|GetPlayerCharacter 0)))
  (Utilities|FlowControl|Sequence
    (:then_0
      ;[1 1 1] Set Card To Visable
      (if (== (Variables|/Game/ThirdPersonBP/Blueprints/Rad_Blueprint.Rad_Blueprint_C|GetTypeofCoin _asrad_blueprint) 0)
        (Rendering|ToggleVisibility (Variables|Default|GetSorry) true)
        ;[1 1 1] If Random Texture is True, Set Random Material
        (if (Variables|Default|GetRandomTexture)
          (switch int (Math|Random|RandomIntegerinRange 0 3)
            (:1
              (Rendering|Material|SetMaterial _sorry 0 "/Game/Geometry/Meshes/Items/Materials/Coin_Sorry1Blue.Coin_Sorry1Blue"))
            (:2
              (Rendering|Material|SetMaterial _sorry 0 "/Game/Geometry/Meshes/Items/Materials/Coin_Sorry2Yellow.Coin_Sorry2Yellow"))
            (:3
              (Rendering|Material|SetMaterial _sorry 0 "/Game/Geometry/Meshes/Items/Materials/Coin_Sorry3Green.Coin_Sorry3Green"))))))
    (:then_1
      ;[1 1 1] Set Pawns to Visable
      (if (== (Variables|/Game/ThirdPersonBP/Blueprints/Rad_Blueprint.Rad_Blueprint_C|GetTypeofCoin _asrad_blueprint) 1)
        (Rendering|ToggleVisibility (Variables|Default|GetCard) true)))
    (:then_2
      ;[1 1 1] Set Letters to Visable
      (if (== (Variables|/Game/ThirdPersonBP/Blueprints/Rad_Blueprint.Rad_Blueprint_C|GetTypeofCoin _asrad_blueprint) 2)
        _))
    (:then_3
      ;[1 1 1] Set Evidence to Visable
      (if (== (Variables|/Game/ThirdPersonBP/Blueprints/Rad_Blueprint.Rad_Blueprint_C|GetTypeofCoin _asrad_blueprint) 3)
        _))
    (:then_4
      ;[1 1 1] Set Dice to Visable
      (if (== (Variables|/Game/ThirdPersonBP/Blueprints/Rad_Blueprint.Rad_Blueprint_C|GetTypeofCoin _asrad_blueprint) 4)
        (Variables|Default|SetDiceOn true)
        (Rendering|ToggleVisibility (Variables|Default|GetDie) true)
        ;[1 1 1] If Random Texture is True, Set Random Material
        (if (Variables|Default|GetRandomTexture)
          (switch int (Math|Random|RandomIntegerinRange 0 5)
            (:1
              (Components|StaticMesh|SetStaticMesh _die "/Game/Geometry/Meshes/Items/Dice/Die_4.Die_4"))
            (:2
              (Components|StaticMesh|SetStaticMesh _die "/Game/Geometry/Meshes/Items/Dice/Die_6.Die_6"))
            (:3
              (Components|StaticMesh|SetStaticMesh _die "/Game/Geometry/Meshes/Items/Dice/Die_8.Die_8"))
            (:4
              (Components|StaticMesh|SetStaticMesh _die "/Game/Geometry/Meshes/Items/Dice/Die_10.Die_10"))
            (:5
              (Components|StaticMesh|SetStaticMesh _die "/Game/Geometry/Meshes/Items/Dice/Die_12.Die_12"))))))))

(fn ConstructionScript)