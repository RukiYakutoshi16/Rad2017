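; Lerp_Cube_Large_BP is an interactible cube actor that moves between its starting location and an offset endpoint.
; On BeginPlay it stores the root's world location as the start and adds the Distance vector to compute the end.
; It then plays the CubeMovement timeline, whose Alpha drives a vector lerp that sets the root's world location without sweep.
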(event EventBeginPlay
  (Utilities|FlowControl|Sequence
    (:then_0
      (Utilities|FlowControl|DoOnce false
        (:Completed
          (Utilities|EndLocationCalculator (Variables|Default|GetDistance)))))
    (:then_1
      (bind _alpha (Timeline|CubeMovement Play)
        (:Update
          (Transformation|SetWorldLocation (Variables|Default|GetDefaultSceneRoot) (Math|Vector|Lerp(Vector) (Variables|Default|GetStartLocation) (Variables|Default|GetEndLocation) _alpha) false false))))))

(event Collision|EventActorBeginOverlap
  (params (OtherActor :type Actor%20Object%20Reference)))

(event EventTick
  (params (DeltaSeconds :type Float%20%28single-precision%29)))

(fn ConstructionScript)